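; TileBuilder is an actor Blueprint that spawns a run of TileBP actors when play begins.
; BeginPlay calls BuildRoom, which spawns MapSize squared tiles at evenly spaced world positions.
; Only X advances with the loop index, so the tiles form a single straight line from the world origin rather than a square grid.
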(event `self.ReceiveBeginPlay`
  (`self.buildRoom`))

(event `self.ReceiveActorBeginOverlap`
  (params (OtherActor :type "Actor Object Reference")))

(event `self.ReceiveTick`
  (params (DeltaSeconds :type "Float (single-precision)")))

(fn `buildRoom`
  (bind _mapsize (`self.mapSize`))
  (for _index (range (* _mapsize _mapsize))
    (`|SpawnActorFromClass` (`self.tileBP`) (`KismetMathLibrary.MakeTransform` (`KismetMathLibrary.MakeVector` (`KismetMathLibrary.Conv_IntToDouble` (* _index 100)))) "Undefined" "OverrideRootScale")))

(fn `UserConstructionScript`)