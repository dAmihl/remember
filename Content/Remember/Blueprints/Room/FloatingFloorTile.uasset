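; FloatingFloorTile is a room floor tile that breaks away once left and can drop to kill the player.
; It extends a parent tile's events: FireAction, for one specific TileType, enables mesh physics and calls KillPlayer on TopDownGameMode.
; OnLeaveTile spawns a physics-simulated FloatingFloorDestructionDummy at the tile's transform if DestructionDummyClass is valid, then always destroys the tile.
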(event `self.ReceiveBeginPlay`
  (`parent.ReceiveBeginPlay`))

(event `self.ReceiveActorBeginOverlap`
  (params (OtherActor :type "Actor Object Reference")))

(event `self.ReceiveTick`
  (params (DeltaSeconds :type "Float (single-precision)"))
  (`parent.ReceiveTick` 0.0))

(event `self.FireAction`
  (`parent.FireAction`)
  (switch `int` (`self.TileType`)
    (:`4`
      (`PrimitiveComponent.SetSimulatePhysics` (`self.StaticMesh`) true)
      (bind _astop_down_game_mode (cast `/Game/Remember/Blueprints/Game/TopDownGameMode` (`GameplayStatics.GetGameMode`)))
      (`/Game/Remember/Blueprints/Game/TopDownGameMode.KillPlayer` _astop_down_game_mode))))

(event `self.OnLeaveTile`
  (`parent.OnLeaveTile`)
  (if (`KismetSystemLibrary.IsValidClass` (`self.DestructionDummyClass`))
    (bind _returnvalue (`|SpawnActorFromClass` "/Game/Remember/Blueprints/Room/FloatingFloorDestructionDummy.FloatingFloorDestructionDummy_C" (`SceneComponent.K2_GetComponentToWorld` (`self.DefaultSceneRoot`)) "Undefined" "OverrideRootScale"))
    (`PrimitiveComponent.SetSimulatePhysics` (`/Game/Remember/Blueprints/Room/RoomTile.StaticMesh` _returnvalue) true))
  (`self.K2_DestroyActor`))

(fn `UserConstructionScript`
  (`parent.UserConstructionScript`))