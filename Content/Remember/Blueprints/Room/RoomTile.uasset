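; RoomTile is a clickable room tile that reports player interaction to the TopDownGameMode.
; Clicks go to the game mode, while FireAction notifies it that the tile is used and also passes the tile to its RoomManager.
; OnLeaveTile flags the tile as already used.
; Tick refreshes a debug label from TileType in test mode, hides it otherwise, and sets its text to USED once flagged.
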(event `self.ReceiveBeginPlay`)

(event `self.ReceiveActorBeginOverlap`
  (params (OtherActor :type "Actor Object Reference")))

(event `self.ReceiveTick`
  (params (DeltaSeconds :type "Float (single-precision)"))
  (`self.updateTextRender`)
  (`self.updateUsedColor`))

(event `self.ReceiveActorOnClicked`
  (`self.onClick`))

(event `onClick`
  (bind _astop_down_game_mode (cast `/Game/Remember/Blueprints/Game/TopDownGameMode` (`GameplayStatics.GetGameMode`)))
  (`/Game/Remember/Blueprints/Game/TopDownGameMode.PlayerClickedTile` _astop_down_game_mode self))

(event `FireAction`
  (bind _astop_down_game_mode (cast `/Game/Remember/Blueprints/Game/TopDownGameMode` (`GameplayStatics.GetGameMode`)))
  (`/Game/Remember/Blueprints/Game/TopDownGameMode.TileUsed` _astop_down_game_mode self)
  (`/Game/Remember/Blueprints/Room/RoomManager.PlayerClickedTile` (`/Game/Remember/Blueprints/Game/TopDownGameMode.RoomManager` _astop_down_game_mode) self))

(event `OnLeaveTile`
  (set `self.alreadyUsed` true))

(fn `updateTextRender`
  (bind _textrender (`self.TextRender`))
  (bind _tiletype (`self.TileType`))
  (bind _astop_down_game_mode (cast `/Game/Remember/Blueprints/Game/TopDownGameMode` (`GameplayStatics.GetGameMode`)))
  (if (`/Game/Remember/Blueprints/Game/TopDownGameMode.TestMode` _astop_down_game_mode)
    (if (!= _tiletype 4)
      (`TextRenderComponent.K2_SetText` _textrender (`KismetTextLibrary.Conv_StringToText` (`KismetStringLibrary.BuildString_Int` "" "" 1)))
      (else
        (`TextRenderComponent.K2_SetText` _textrender (`KismetTextLibrary.Conv_StringToText` (`KismetStringLibrary.BuildString_Int` "" "" _tiletype)))))
    (else
      (`SceneComponent.SetVisibility` _textrender false false))))

(fn `updateUsedColor`
  (if (`self.alreadyUsed`)
    (`TextRenderComponent.K2_SetText` (`self.TextRender`) (`KismetTextLibrary.Conv_StringToText` (`KismetStringLibrary.Concat_StrStr` "USED")))))

(fn `UserConstructionScript`)