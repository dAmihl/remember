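; Timed variant of a floating floor tile that falls down after a delay once its action fires.
; It overrides FireAction, runs the parent behavior, then starts a one-shot timer using TimeToFall.
; When the timer expires, a custom event calls TileFallDown to drop the tile.
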(event `self.ReceiveBeginPlay`
  (`parent.ReceiveBeginPlay`))

(event `self.ReceiveActorBeginOverlap`
  (params (OtherActor :type "Actor Object Reference")))

(event `self.ReceiveTick`
  (params (DeltaSeconds :type "Float (single-precision)"))
  (`parent.ReceiveTick` 0.0))

(event `timedFallDown`
  (`self.TileFallDown`))

(event `/Game/Remember/Blueprints/Room/RoomTile.FireAction`
  (`parent.FireAction`)
  (`KismetSystemLibrary.K2_SetTimerDelegate` (delegate `timedFallDown`) (`self.timeToFall`)))

(fn `UserConstructionScript`
  (`parent.UserConstructionScript`))