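; Room manager that spawns the game's rooms from 4x4 matrices and tracks the active one.
; The first room uses a random matrix, cached for rebuilds, and resets the game mode's room number.
; Every clicked tile, regardless of type, queues its transposed tile matrix; the next room's matrix is the product of that queue in click order.
; It also forwards player death to the game mode.
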(event EventBeginPlay
  (CallFunction|BuildFirstRoom))

(event EventActorBeginOverlap
  (params (OtherActor :type Actor%20Object%20Reference)))

(event EventTick
  (params (DeltaSeconds :type Float%20%28single-precision%29)))

(event Custom|PlayerClickedTile
  (params (Tile :type Room%20Tile%20Object%20Reference))
  (switch int (Variables|/Game/Remember/Blueprints/Room/RoomTile.RoomTile_C|GetTileType Tile)
    (:Default
      _)
    (:0
      _)
    (:1
      _)
    (:2
      _)
    (:3
      _))
  (bind _returnvalue (Class|Mat4|TileMatrix (Variables|Default|GetRoomMatrix) (Utilities|Array|FindItem (Variables|/Game/Remember/Blueprints/Room/Room.Room_C|GetTiles (Variables|Default|GetactiveRoom)) Tile)))
  (Class|Mat4|Transpose _returnvalue)
  (Utilities|Array|Add (Variables|Default|GettileMats) _returnvalue))

(fn ConstructionScript)

(fn BuildFirstRoom
  (Utilities|IsValid (Variables|Default|GetInitialMatrix)
    (:Is%20Valid
      ;[1 1 1] Initial matrix is already set and can be used
      (bind _returnvalue (Game|SpawnActorfromClass "/Game/Remember/Blueprints/Room/Room.Room_C" (Math|Transform|MakeTransform (Transformation|GetActorLocation)) "Undefined" 0 0))
      (bind _output_get (Variables|Default|SetRoomMatrix (Variables|Default|GetInitialMatrix)))
      (Default|StartConstruction _returnvalue _output_get)
      (Variables|Default|SetactiveRoom _returnvalue)
      (Utilities|Array|Clear (Variables|Default|GettileMats))
      (bind _astop_down_game_mode (Utilities|Casting|CastToTopDownGameMode (Game|GetGameMode)))
      (Variables|/Game/Remember/Blueprints/Game/TopDownGameMode.TopDownGameMode_C|SetRoomNumber _astop_down_game_mode 1)
      (return 0))
    (:Is%20Not%20Valid
      ;[1 1 1] The first time the first room gets created. Initial matrix is not set yet.
      (bind _returnvalue_2 (Game|SpawnActorfromClass "/Script/Remember.Mat4" (LocalVariables|GetspawnTransform) "Undefined" 0 0))
      (Class|Mat4|MakeRandomMatrix _returnvalue_2)
      (bind _returnvalue_3 (Game|SpawnActorfromClass "/Game/Remember/Blueprints/Room/Room.Room_C" (Math|Transform|MakeTransform (Transformation|GetActorLocation)) "Undefined" 0 0))
      (bind _output_get_2 (Variables|Default|SetInitialMatrix _returnvalue_2))
      (bind _output_get_3 (Variables|Default|SetRoomMatrix _output_get_2))
      (Default|StartConstruction _returnvalue_3 _output_get_3)
      (Variables|Default|SetactiveRoom _returnvalue_3)
      (Utilities|Array|Clear (Variables|Default|GettileMats))
      (bind _astop_down_game_mode_2 (Utilities|Casting|CastToTopDownGameMode (Game|GetGameMode)))
      (Variables|/Game/Remember/Blueprints/Game/TopDownGameMode.TopDownGameMode_C|SetRoomNumber _astop_down_game_mode_2 1)
      (return _returnvalue_3))))

(fn BuildNextRoom
  (bind _newroommatrix (CallFunction|ComputeNewMatrix))
  (bind _returnvalue (Game|SpawnActorfromClass "/Game/Remember/Blueprints/Room/Room.Room_C" (Math|Transform|MakeTransform (Transformation|GetActorLocation)) "Undefined" 0 0))
  (bind _output_get (Variables|Default|SetRoomMatrix _newroommatrix))
  (Default|StartConstruction _returnvalue _output_get)
  (Variables|Default|SetactiveRoom _returnvalue)
  (Utilities|Array|Clear (Variables|Default|GettileMats))
  (return _returnvalue))

(fn ComputeNewMatrix
  (bind _tilemats (Variables|Default|GettileMats))
  (LocalVariables|SettmpMat (Utilities|Array|Get(acopy) _tilemats))
  (Utilities|Array|RemoveIndex _tilemats)
  (for _array_element _tilemats
    (bind _returnvalue (Class|Mat4|Multiply (LocalVariables|GettmpMat) _array_element))
    (LocalVariables|SettmpMat _returnvalue))
  (return (LocalVariables|GettmpMat)))

(fn KillPlayer
  (bind _astop_down_game_mode (Utilities|Casting|CastToTopDownGameMode (Game|GetGameMode)))
  (Default|KillPlayer _astop_down_game_mode))