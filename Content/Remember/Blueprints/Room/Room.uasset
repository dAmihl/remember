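; Room actor that forms a tile-based level section and handles click-to-move for the player.
; StartConstruction spawns a four-column grid of typed RoomTiles from a room matrix, plus an ExitTile one tile beyond the last, centered on Y.
; Clicked tiles within range teleport the controlled pawn above them, otherwise a message prints.
; Destroying the room also destroys all its tiles.
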(event EventBeginPlay)

(event EventActorBeginOverlap
  (params (OtherActor :type Actor%20Object%20Reference)))

(event EventTick
  (params (DeltaSeconds :type Float%20%28single-precision%29)))

(event EventDestroyed
  (for _array_element (Variables|Default|GetTiles)
    (Actor|DestroyActor _array_element)))

(event Custom|PlayerClickedTile
  (params (Tile :type Room%20Tile%20Object%20Reference))
  (if (CallFunction|TileIsReachable Tile)
    (CallFunction|MovePlayertoTile Tile)
    (else
      (Development|PrintString "Tile not reachable!"))))

(fn ConstructionScript)

(fn StartConstruction
  (params (RoomMatrix :type Mat%204%20Object%20Reference))
  (bind _returnvalue (Class|Mat4|GetMatrix RoomMatrix))
  (for (_array_element _array_index) _returnvalue
    (bind _output_get (LocalVariables|SetspawnX (* (Math|Integer|%(Integer) _array_index 4) (Variables|Default|GetTileSize))))
    (bind _output_get_2 (LocalVariables|SetspawnY (* (/ _array_index 4) (Variables|Default|GetTileSize))))
    (bind _returnvalue_2 (Game|SpawnActorfromClass "/Game/Remember/Blueprints/Room/RoomTile.RoomTile_C" (Math|Transform|MakeTransform (+ (Transformation|GetActorLocation) (Math|Vector|MakeVector (Math|Conversions|ToFloat(Integer) _output_get) (Math|Conversions|ToFloat(Integer) _output_get_2) 0.0))) "Undefined" 0 0))
    (Variables|/Game/Remember/Blueprints/Room/RoomTile.RoomTile_C|SetTileType _returnvalue_2 _array_element)
    (Utilities|Array|Add (Variables|Default|GetTiles) _returnvalue_2)
    (Variables|/Game/Remember/Blueprints/Room/RoomTile.RoomTile_C|SetassociatedRoom _returnvalue_2 self)
    (LocalVariables|Setlast%20spawn (+ (Transformation|GetActorLocation) (Math|Vector|MakeVector (Math|Conversions|ToFloat(Integer) _output_get) (Math|Conversions|ToFloat(Integer) _output_get_2) 0.0))))
  (bind _returnvalue_3 (Class|GameplayStatics|GetActorArrayAverageLocation (Variables|Default|GetTiles)))
  (bind _returnvalue_4 (Game|SpawnActorfromClass "/Game/Remember/Blueprints/Room/ExitTile.ExitTile_C" (Math|Conversions|ToTransform(Vector) (Math|Vector|MakeVector (.x (+ (LocalVariables|Getlast%20spawn) (Math|Vector|MakeVector (Math|Conversions|ToFloat(Integer) (Variables|Default|GetTileSize)) 0.0 0.0))) (.y _returnvalue_3) 0.0)) "Undefined" 0 0))
  (Variables|/Game/Remember/Blueprints/Room/RoomTile.RoomTile_C|SetassociatedRoom _returnvalue_4 self)
  (Utilities|Array|Add (Variables|Default|GetTiles) _returnvalue_4))

(fn TileIsReachable
  (params (tile :type Room%20Tile%20Object%20Reference))
  (return (<= (Transformation|GetDistanceTo (Pawn|GetControlledPawn (Game|GetPlayerController 0)) tile) (+ (Math|Conversions|ToFloat(Integer) (Variables|Default|GetTileSize)) (Math|Conversions|ToFloat(Integer) (Variables|Default|GetmovementDistance))))))

(fn MovePlayertoTile
  (params (toTile :type Room%20Tile%20Object%20Reference))
  (Transformation|SetActorLocation (Pawn|GetControlledPawn (Game|GetPlayerController 0)) (+ (Transformation|GetActorLocation toTile) "0, 0,100.000000") false false))